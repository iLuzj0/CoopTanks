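; Spawner component for a procedural dungeon, meant to place items or enemies on floor tiles but apparently unfinished.
; It caches its owning BP_ProceduralDungeonGenerator on BeginPlay, and TrigerSpawnEnemies copies that dungeon's floor tiles without calling SpawnItems.
; SpawnItems picks random tile indices from the dungeon's seeded stream, but nothing spawns, its loop never increments ItemsSpawned, and the world-location math is unconnected.
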(event Custom|TrigerSpawnEnemies
  (Variables|Default|SetFloor%20Tiles (Variables|/Game/Blueprints/Actors/BP_ProceduralDungeonGenerator.BP_ProceduralDungeonGenerator_C|GetFloor%20Tiles (Variables|Default|GetDungeon))))

(event EventBeginPlay
  (bind _asbp_procedural_dungeon_generator (Utilities|Casting|CastToBP_ProceduralDungeonGenerator (Components|GetOwner)))
  (Variables|Default|SetDungeon _asbp_procedural_dungeon_generator))

(fn SpawnItems
  (while (> (Variables|Default|GetQuantity) (LocalVariables|GetItemsSpawned))
    (LocalVariables|SetFloorIndex (Math|Random|RandomIntegerinRangefromStream 0 (Utilities|Array|LastIndex (Variables|Default|GetFloor%20Tiles)) (Variables|/Game/Blueprints/Actors/BP_ProceduralDungeonGenerator.BP_ProceduralDungeonGenerator_C|GetStream (Variables|Default|GetDungeon))))))