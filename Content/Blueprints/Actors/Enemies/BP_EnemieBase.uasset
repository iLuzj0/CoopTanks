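; Base enemy turret that turns toward player-tagged actors within a box range, turns its sphere red and fires railgun projectiles at a GameState-driven rate.
; Bullet overlaps on Capsule and Box proportionally reduce separate tower and weapon health, with a random chance of rage at low health that only recolors that part red.
; When both healths reach zero, a timeline-driven material dissolve destroys the actor, which notifies GameState.
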(event OnComponentBeginOverlap(Capsule)
  (params (OverlappedComponent :type Primitive%20Component%20Object%20Reference) (OtherActor :type Actor%20Object%20Reference) (OtherComp :type Primitive%20Component%20Object%20Reference) (OtherBodyIndex :type Integer) (bFromSweep :type Boolean) (SweepResult :type Hit%20Result%20Structure%20%28by%20ref%29))
  (if (Actor|ActorHasTag OtherActor "Bullet")
    (bind _output_get (Variables|Default|SetTowerHealth (- (Variables|Default|GetTowerHealth) (/ (Variables|Default|GetTowerHealth) (Variables|/Game/ModularLowPolyRobots/Blueprints/BP_GameState.BP_GameState_C|GetEnemieTowerHits (Variables|Default|GetGameState))))))
    (if (and (<= _output_get 0.2) (Math|Random|RandomBoolwithWeight (Variables|Difficulty|GetRageChance)))
      (Utilities|FlowControl|DoOnce false
        (:Completed
          (CallFunction|EnterTowerRage))))))

(event OnComponentBeginOverlap(Box)
  (params (OverlappedComponent :type Primitive%20Component%20Object%20Reference) (OtherActor :type Actor%20Object%20Reference) (OtherComp :type Primitive%20Component%20Object%20Reference) (OtherBodyIndex :type Integer) (bFromSweep :type Boolean) (SweepResult :type Hit%20Result%20Structure%20%28by%20ref%29))
  (if (Actor|ActorHasTag OtherActor "Bullet")
    (bind _output_get (Variables|Default|SetWeaponHealth (- (Variables|Default|GetWeaponHealth) (/ (Variables|Default|GetWeaponHealth) (Variables|/Game/ModularLowPolyRobots/Blueprints/BP_GameState.BP_GameState_C|GetEnemieWaponHIts (Variables|Default|GetGameState))))))
    (if (and (<= _output_get 0.2) (Math|Random|RandomBoolwithWeight (Variables|Difficulty|GetRageChance)))
      (Utilities|FlowControl|DoOnce false
        (:Completed
          (CallFunction|EnterWeaponRage))))))

(event Custom|DisolveActor
  (bind _returnvalue (Rendering|Material|CreateDynamicMaterialInstance "/Game/Blueprints/Materials/MaterialInstances/MI_EnemiesDestruction.MI_EnemiesDestruction" "None" "None" :!class /Script/Engine.KismetMaterialLibrary))
  (Variables|Default|SetDestructionMaterial _returnvalue)
  (Rendering|Material|SetMaterial (Variables|Default|GetGun) 0 (Variables|Default|GetDestructionMaterial))
  (Rendering|Material|SetMaterial (Variables|Default|GetGun) 1 (Variables|Default|GetDestructionMaterial))
  (bind _destroy (Timeline|DestroyAnim Play)
    (:Update
      (Rendering|Material|SetScalarParameterValue (Variables|Default|GetDestructionMaterial) "Appearance" _destroy :!class /Script/Engine.MaterialInstanceDynamic))
    (:Finished
      (Actor|DestroyActor))))

(event Custom|EnterWeaponRage
  ;[1 0 0.6094] EnterWeaponRage
  (Rendering|Material|SetMaterial (Variables|Default|GetGun) 1 "/Game/ModularLowPolyRobots/Materials/ColorMaterialsInstances/MI_ColorRed.MI_ColorRed"))

(event Custom|EnterTowerRage
  ;[1 0 0.7734] EnterTowerRage
  (Rendering|Material|SetMaterial (Variables|Default|GetStaticMesh) 0 "/Game/ModularLowPolyRobots/Materials/ColorMaterialsInstances/MI_ColorRed.MI_ColorRed"))

(event Custom|Shoot
  (bind _gun (Variables|Default|GetGun))
  (Utilities|FlowControl|Delay (/ 1.0 (Variables|/Game/ModularLowPolyRobots/Blueprints/BP_GameState.BP_GameState_C|GetEnemieFireRate (Variables|Default|GetGameState))))
  (bind _returnvalue (Game|SpawnActorfromClass "/Game/Blueprints/Projectiles/BP_RailGunProjectile.BP_RailGunProjectile_C" (Math|Transform|MakeTransform (Transformation|GetSocketLocation _gun "ShootSocket") (Transformation|GetWorldRotation _gun) "1,1,1") "Undefined" 0 0))
  (Variables|/Script/Engine.Actor|SetTags _returnvalue (Utilities|Array|MakeArray "EnemieBullet")))

(event EventTick
  (params (DeltaSeconds :type Float%20%28single-precision%29))
  (bind _returnvalue (Transformation|GetActorLocation))
  (Variables|Default|SetDeltaTime DeltaSeconds)
  (if (and (<= (Variables|Default|GetTowerHealth) 0.0) (<= (Variables|Default|GetWeaponHealth) 0.0))
    (Utilities|FlowControl|DoOnce false
      (:Completed
        (CallFunction|DisolveActor)))
    (else
      (bind _outactors (Actor|GetAllActorswithTag "player"))
      (bind _output_get (Variables|Default|SetPlayerActors _outactors))
      (for _array_element _output_get
        (if (Math|Geometry|IsPointinBox (Transformation|GetActorLocation _array_element) _returnvalue "3500.000000,3500.000000,10000.000000")
          (Transformation|SetActorRotation (Math|Interpolation|RInterpTo (Transformation|GetActorRotation) (Math|Rotator|MakeRotator 0.0 0.0 (.yaw (Math|Rotator|FindLookatRotation _returnvalue (Transformation|GetActorLocation _array_element)))) (Variables|Default|GetDeltaTime) (* (Variables|/Game/ModularLowPolyRobots/Blueprints/BP_GameState.BP_GameState_C|GetTowerTurningSpeed (Variables|Default|GetGameState)) 0.4)))
          (Rendering|Material|SetMaterial (Variables|Default|GetSphere) 0 "/Game/ModularLowPolyRobots/Materials/ColorMaterialsInstances/MI_ColorRed.MI_ColorRed")
          (CallFunction|Shoot)
          (else
            (Rendering|Material|SetMaterial (Variables|Default|GetSphere) 0 "/Game/ModularLowPolyRobots/Materials/ColorMaterialsInstances/MI_ColorGreen.MI_ColorGreen")))))))

(event EventDestroyed
  (Default|EnemieDies (Variables|Default|GetGameState)))

(event EventBeginPlay
  (bind _asbp_game_state (Utilities|Casting|CastToBP_GameState (Game|GetGameState)))
  (Variables|Default|SetGameState _asbp_game_state))

(fn ConstructionScript)