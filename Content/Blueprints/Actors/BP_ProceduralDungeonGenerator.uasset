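; Procedural dungeon generator actor that builds a tile-grid room layout from a seeded random stream on BeginPlay.
; Rooms step out from the previous one in eight directions, restarting from a random earlier room when blocked or optionally branching.
; Optional culling randomly removes tiles, using a flood fill to keep a large enough connected area.
; SpawnTiles adds instanced floors, walls and outer corners by testing each tile's neighbours.
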(event Custom|GenerateMap
  ;[1 0 0.375] GenerateMap
  (for _index (range 0 (- (Variables|MapSettings|GetRoomCount) 1))
    (if (== _index 0)
      (CallFunction|SetupFirstRoom)
      (elif (Variables|MapSettings|GetBranching)
        (CallFunction|CanRoomBranch)
        (else
          (CallFunction|CreateNextRooms)))))
  (CallFunction|SpawnTiles))

(event Custom|CreateNextRooms
  ;[0.9219 0 1] Find location to place next room and calculate floor tiles for new room if room fails to be found force to use one of previously created rooms
  (bind (_isvalid _outlocation) (RoomSetup|RoomFindNextLocation))
  (if _isvalid
    (bind _output_get (Variables|Default|SetNextLocation _outlocation))
    (bind (_floortiles _floorlocation _extents) (RoomSetup|RoomMakeFloorArea _output_get))
    (Utilities|Array|AppendArray (Variables|Default|GetFloor%20Tiles) _floortiles)
    (Utilities|Map|Add (Variables|Default|GetRooms) _floorlocation _extents)
    (Variables|Default|SetPrevLocation (Variables|Default|GetNextLocation))
    (else
      (CallFunction|GetAlreadyCreatedRoom))))

(event Custom|GetAlreadyCreatedRoom
  ;[0 0.5547 1] Get precious room to branch from
  (bind _keys (Utilities|Map|Keys (Variables|Default|GetRooms)))
  (Variables|Default|SetPrevLocation (Utilities|Array|Get(acopy) _keys (Class|KismetMathLibrary|RandomIntegerfromStream (Utilities|Array|LastIndex _keys) (Variables|Default|GetStream))))
  (Variables|Default|SetLastBranch (Class|KismetMathLibrary|RandomIntegerfromStream (Utilities|Array|LastIndex _keys) (Variables|Default|GetStream)))
  (CallFunction|CreateNextRooms))

(event Custom|CanRoomBranch
  ;[0 0.1797 1] Can and will the room branch from previous
  (bind _keys (Utilities|Map|Keys (Variables|Default|GetRooms)))
  (if (and (>= (Utilities|Array|LastIndex _keys) (+ (Variables|MapSettings|GetBranchingThreshold) (Variables|Default|GetLastBranch))) (Class|KismetMathLibrary|RandomBoolwithWeightfromStream (Variables|MapSettings|GetBranchingChance) (Variables|Default|GetStream)))
    (CallFunction|GetAlreadyCreatedRoom)
    (else
      (CallFunction|CreateNextRooms))))

(event Custom|SetupFirstRoom
  ;[0 1 0.6953] SetupFirstRoom
  (bind (_floortiles _floorlocation _extents) (RoomSetup|RoomMakeFloorArea (Variables|Default|GetPrevLocation)))
  (Variables|Default|SetFloor%20Tiles _floortiles)
  (Utilities|Map|Add (Variables|Default|GetRooms) _floorlocation _extents))

(event EventBeginPlay
  ;[1 0.7266 0] Begin play
  ;;[0.3359 0 1] SetRandomSeedManually
  (Math|Random|SetRandomStreamSeed (Variables|Default|GetStream) (Variables|MapSettings|GetSeed))
  (CallFunction|GenerateMap))

(fn ConstructionScript)

(fn RoomMakeFloorArea
  (params (Location :type Int%20Vector%20Structure))
  ;[0.8984 1 0] Generate X and Y coords and make tiles array for floor
  (LocalVariables|SetRootLocation Location)
  (LocalVariables|SetOutX (Math|Random|RandomIntegerinRangefromStream (Variables|MapSettings|GetRoomSizeMin) (Variables|MapSettings|GetRoomSizeMax) (Variables|Default|GetStream)))
  (LocalVariables|SetOutY (Math|Random|RandomIntegerinRangefromStream (Variables|MapSettings|GetRoomSizeMin) (Variables|MapSettings|GetRoomSizeMax) (Variables|Default|GetStream)))
  (for _index (range 0 (- (* (LocalVariables|GetOutX) (LocalVariables|GetOutY)) 1))
    (Utilities|Array|Add (LocalVariables|GetTiles) (Utilities|Struct|MakeIntVector (+ (/ _index (LocalVariables|GetOutY)) (.x (LocalVariables|GetRootLocation))) (+ (Math|Integer|%(Integer) _index (LocalVariables|GetOutY)) (.y (LocalVariables|GetRootLocation))) (.z (LocalVariables|GetRootLocation)))))
  (if (Variables|MapSettings|GetIsFloorCulling)
    (while (LocalVariables|GetWorking)
      (if (<= (LocalVariables|GetLoopCount) (Variables|EditorTools|GetMaxLoops))
        ;[0.7344 0 1] Randomly remove tiles from the floor
        (LocalVariables|SetTilesCopy (LocalVariables|GetTiles))
        (for _index_2 (range 0 (Math|Integer|Clamp(Integer) (- (Math|Random|RandomIntegerinRangefromStream (Variables|MapSettings|GetFloorCullMin) (Variables|MapSettings|GetFloorCullMax) (Variables|Default|GetStream)) 1) 0 (/ (Utilities|Array|Length (LocalVariables|GetTilesCopy)) 4)))
          (Utilities|Array|RemoveIndex (LocalVariables|GetTilesCopy) (Class|KismetMathLibrary|RandomIntegerfromStream (Utilities|Array|LastIndex (LocalVariables|GetTilesCopy)) (Variables|Default|GetStream))))
        ;[1 0 0.3516] Testing if addjustment tiles are present if so add to connected tile array
        (Utilities|Array|Clear (LocalVariables|GetConnectedTiles))
        (Utilities|Array|Add (LocalVariables|GetConnectedTiles) (Utilities|Array|Get(acopy) (LocalVariables|GetTilesCopy)))
        (while (LocalVariables|GetFoundTile)
          (LocalVariables|SetFoundTile false)
          (for _array_element (LocalVariables|GetConnectedTiles)
            (for _index_3 (range 0 3)
              (if (Utilities|Select :Index _index_3 :Option%200 (.LocationExists (Utilities|TestRelativeTileLocation _array_element (LocalVariables|GetTilesCopy) 1)) :Option%201 (.LocationExists (Utilities|TestRelativeTileLocation _array_element (LocalVariables|GetTilesCopy) 0 1)) :Option%202 (.LocationExists (Utilities|TestRelativeTileLocation _array_element (LocalVariables|GetTilesCopy) -1)) :Option%203 (.LocationExists (Utilities|TestRelativeTileLocation _array_element (LocalVariables|GetTilesCopy) 0 -1)))
                (Utilities|Array|Add (LocalVariables|GetConnectedTiles) (Utilities|Select :Index _index_3 :Option%200 (.Location (Utilities|TestRelativeTileLocation _array_element (LocalVariables|GetTilesCopy) 1)) :Option%201 (.Location (Utilities|TestRelativeTileLocation _array_element (LocalVariables|GetTilesCopy) 0 1)) :Option%202 (.Location (Utilities|TestRelativeTileLocation _array_element (LocalVariables|GetTilesCopy) -1)) :Option%203 (.Location (Utilities|TestRelativeTileLocation _array_element (LocalVariables|GetTilesCopy) 0 -1))))
                (Utilities|Array|RemoveItem (LocalVariables|GetTilesCopy) (Utilities|Select :Index _index_3 :Option%200 (.Location (Utilities|TestRelativeTileLocation _array_element (LocalVariables|GetTilesCopy) 1)) :Option%201 (.Location (Utilities|TestRelativeTileLocation _array_element (LocalVariables|GetTilesCopy) 0 1)) :Option%202 (.Location (Utilities|TestRelativeTileLocation _array_element (LocalVariables|GetTilesCopy) -1)) :Option%203 (.Location (Utilities|TestRelativeTileLocation _array_element (LocalVariables|GetTilesCopy) 0 -1))))))))
        ;[0.8047 0 1] Is array of connected tiles larger than minimum area if not try again and increment loop count
        (if (> (Utilities|Array|Length (LocalVariables|GetConnectedTiles)) (* (Variables|MapSettings|GetRoomSizeMin) (Variables|MapSettings|GetRoomSizeMax)))
          (LocalVariables|SetWorking false)
          (else
            (LocalVariables|SetWorking true)
            (Math|Integer|IncrementInt (LocalVariables|GetLoopCount))))
        (else
          ;[0 0.8125 1] Failed out without culling tiles
          (LocalVariables|SetWorking false)
          (LocalVariables|SetConnectedTiles (LocalVariables|GetTiles)))))
    (else
      (LocalVariables|SetConnectedTiles (LocalVariables|GetTiles))))
  ;[0 0.08594 1] Get outer extents of room and output final results
  (for _array_element_2 (LocalVariables|GetConnectedTiles)
    (Utilities|Array|Add (LocalVariables|GetExtentsX) (.X (Utilities|Struct|BreakIntVector _array_element_2)))
    (Utilities|Array|Add (LocalVariables|GetExtentsY) (.Y (Utilities|Struct|BreakIntVector _array_element_2))))
  (return (LocalVariables|GetConnectedTiles) (LocalVariables|GetRootLocation) (Utilities|Struct|MakeIntVector (.MaxValue (Math|Integer|MaxOfIntArray (LocalVariables|GetExtentsX))) (.MaxValue (Math|Integer|MaxOfIntArray (LocalVariables|GetExtentsY))))))

(fn SpawnTiles
  (for _array_element (Variables|Default|GetFloor%20Tiles)
    (Utilities|FlowControl|Sequence
      (:then_0
        ;[1 0.2578 0] Generate floor
        (Components|InstancedStaticMesh|AddInstance (Variables|Default|GetFloor) (Math|Transform|MakeTransform (* (Math|Conversions|ToVector(Float) _array_element) (Variables|EditorTools|GetScale)) "0, 0, 0" "1,1,1")))
      (:then_1
        ;[0 1 0.3203] Generate walls
        (for _index (range 0 3)
          (if (not (Utilities|Select :Index _index :Option%200 (.LocationExists (Utilities|TestRelativeTileLocation _array_element (Variables|Default|GetFloor%20Tiles) 1)) :Option%201 (.LocationExists (Utilities|TestRelativeTileLocation _array_element (Variables|Default|GetFloor%20Tiles) 0 1)) :Option%202 (.LocationExists (Utilities|TestRelativeTileLocation _array_element (Variables|Default|GetFloor%20Tiles) -1)) :Option%203 (.LocationExists (Utilities|TestRelativeTileLocation _array_element (Variables|Default|GetFloor%20Tiles) 0 -1))))
            (Components|InstancedStaticMesh|AddInstance (Variables|Default|GetWalls) (Math|Transform|MakeTransform (* (Math|Conversions|ToVector(Float) _array_element) (Variables|EditorTools|GetScale)) (Utilities|Select :Index _index :Option%200 "0, 0, 0" :Option%201 "0.000000,90.000000, 0" :Option%202 "0.000000,180.000000, 0" :Option%203 "0.000000,-90.000000, 0") "1,1,1")))))
      (:then_2
        ;[1 0 0.9375] Generate outer corners
        (for _index_2 (range 0 3)
          (if (Utilities|Select :Index _index_2 :Option%200 (and (not (.LocationExists (Utilities|TestRelativeTileLocation _array_element (Variables|Default|GetFloor%20Tiles) 1 -1))) (and (.LocationExists (Utilities|TestRelativeTileLocation _array_element (Variables|Default|GetFloor%20Tiles) 1)) (.LocationExists (Utilities|TestRelativeTileLocation _array_element (Variables|Default|GetFloor%20Tiles) 0 -1)))) :Option%201 (and (not (.LocationExists (Utilities|TestRelativeTileLocation _array_element (Variables|Default|GetFloor%20Tiles) 1 1))) (and (.LocationExists (Utilities|TestRelativeTileLocation _array_element (Variables|Default|GetFloor%20Tiles) 1)) (.LocationExists (Utilities|TestRelativeTileLocation _array_element (Variables|Default|GetFloor%20Tiles) 0 1)))) :Option%202 (and (not (.LocationExists (Utilities|TestRelativeTileLocation _array_element (Variables|Default|GetFloor%20Tiles) -1 1))) (and (.LocationExists (Utilities|TestRelativeTileLocation _array_element (Variables|Default|GetFloor%20Tiles) -1)) (.LocationExists (Utilities|TestRelativeTileLocation _array_element (Variables|Default|GetFloor%20Tiles) 0 1)))) :Option%203 (and (not (.LocationExists (Utilities|TestRelativeTileLocation _array_element (Variables|Default|GetFloor%20Tiles) -1 -1))) (and (.LocationExists (Utilities|TestRelativeTileLocation _array_element (Variables|Default|GetFloor%20Tiles) -1)) (.LocationExists (Utilities|TestRelativeTileLocation _array_element (Variables|Default|GetFloor%20Tiles) 0 -1)))))
            (Components|InstancedStaticMesh|AddInstance (Variables|Default|GetOuterCorners) (Math|Transform|MakeTransform (* (Math|Conversions|ToVector(Float) _array_element) (Variables|EditorTools|GetScale)) (Utilities|Select :Index _index_2 :Option%200 "0, 0, 0" :Option%201 "0.000000,90.000000, 0" :Option%202 "0.000000,180.000000, 0" :Option%203 "0.000000,-90.000000, 0") "1,1,1"))))))))

(fn RoomFindNextLocation
  (LocalVariables|SetDirections (Utilities|Array|MakeArray 0 1 2 3 4 5 6 7))
  (while (LocalVariables|GetSearching)
    (if (>= (Utilities|Array|LastIndex (LocalVariables|GetDirections)) 0)
      (bind _output_get (LocalVariables|SetTestIndex (Class|KismetMathLibrary|RandomIntegerfromStream (Utilities|Array|LastIndex (LocalVariables|GetDirections)) (Variables|Default|GetStream))))
      (if (.IsFloorTile (Utilities|CheckforLocationColisions (Variables|Default|GetPrevLocation) (Variables|Default|GetFloor%20Tiles) (Variables|MapSettings|GetRoomSizeMax) _output_get))
        (Utilities|Array|RemoveIndex (LocalVariables|GetDirections) (LocalVariables|GetTestIndex))
        (LocalVariables|SetSearching true)
        (else
          (LocalVariables|SetSearching false)
          (LocalVariables|SetValid true)
          (LocalVariables|SetNewLocation (.OutLocation (Utilities|CheckforLocationColisions (Variables|Default|GetPrevLocation) (Variables|Default|GetFloor%20Tiles) (Variables|MapSettings|GetRoomSizeMax) _output_get)))))
      (else
        (LocalVariables|SetSearching false)
        (LocalVariables|SetValid false))))
  (return (LocalVariables|GetValid) (LocalVariables|GetNewLocation)))