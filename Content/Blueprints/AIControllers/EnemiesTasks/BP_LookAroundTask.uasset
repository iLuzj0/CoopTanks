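; Behavior tree task that makes an enemy appear to look around by swinging its gun toward random points.
; On AI execute, it rotates the BP_EnemieBase pawn's Gun component toward a random point in a box around the pawn, then repeats after a short delay.
; The loop has no exit and never calls Finish Execute.
; A SetFocalPoint call is left unconnected.
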(event EventReceiveExecuteAI
  (params (OwnerController :type AI%20Controller%20Object%20Reference) (ControlledPawn :type Pawn%20Object%20Reference))
  (Variables|Default|SetOwner%20Controller OwnerController)
  (bind _output_get (Variables|Default|SetControlled%20Pawn ControlledPawn))
  (Transformation|SetWorldRotation (Variables|/Game/Blueprints/Actors/Enemies/BP_EnemieBase.BP_EnemieBase_C|GetGun (.AsBP%20Enemie%20Base (Utilities|Casting|CastToBP_EnemieBase _output_get))) (Math|Rotator|FindLookatRotation (Transformation|GetActorLocation (.AsBP%20Enemie%20Base (Utilities|Casting|CastToBP_EnemieBase _output_get))) (Math|Random|RandomPointinBoundingBox (Transformation|GetActorLocation (Pawn|GetControlledPawn (Variables|Default|GetOwner%20Controller))) "200.000000,200.000000,200.000000")) false false :!label _label)
  (Utilities|FlowControl|Delay 2.0)
  (goto _label))