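; Player controller for the modular robots demo that starts BP_RobotSpawner pawns from key, gamepad or network OSC input.
; BeginPlay opens an OSC server on port 8000, whose "/MoveForward" message calls InitStart on player 0's spawner.
; Key 1 does the same, while gamepad Special Right starts player 1's spawner.
; Tab and Escape share a demo menu toggle, but the widget creation nodes are disconnected, leaving DemoMenu unassigned here.
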(event Custom|OSCMessageReceived
  (params (Message :type OSC%20Message%20Structure%20%28by%20ref%29) (IPAddress :type String) (Port :type Integer))
  (bind _returnvalue (Class|OSCManager|GetOSCMessageAddress Message))
  (bind _returnvalue_2 (Class|OSCManager|GetOSCAddressFullPath _returnvalue))
  (if (Utilities|Enum|Equal(Enum) _returnvalue_2 "/MoveForward")
    (bind _asbp_robot_spawner (Utilities|Casting|CastToBP_RobotSpawner (Game|Player|GetPlayerPawn 0)))
    (Default|InitStart _asbp_robot_spawner)))

(event EventBeginPlay
  (bind _returnvalue (Class|OSCManager|CreateOSCServer "0.0.0.0" 8000 false true "" 0))
  (bind _output_get (Variables|Default|SetOSCServer _returnvalue))
  (EventDispatchers|UnbindallEventsfromOnOscBundleReceived _output_get)
  (EventDispatchers|BindEventtoOnOscMessageReceived _output_get (EventDispatchers|CreateEvent :!event Custom|OSCMessageReceived)))

(event Input|KeyboardEvents|Tab
  (params (Key :type Key%20Structure :default "None"))
  (bind _demomenu (Variables|Default|GetDemoMenu))
  (:Pressed
    (Utilities|FlowControl|FlipFlop
      (:A
        (Default|ShowWidget _demomenu true))
      (:B
        (Default|ShowWidget _demomenu false)))))

(event Input|KeyboardEvents|Escape
  (params (Key :type Key%20Structure :default "None"))
  (bind _demomenu (Variables|Default|GetDemoMenu))
  (:Pressed
    (Utilities|FlowControl|FlipFlop
      (:A
        (Default|ShowWidget _demomenu true))
      (:B
        (Default|ShowWidget _demomenu false)))))

(event Input|GamepadEvents|GamepadSpecialRight
  (params (Key :type Key%20Structure :default "None"))
  (:Pressed
    (bind _asbp_robot_spawner (Utilities|Casting|CastToBP_RobotSpawner (Game|Player|GetPlayerPawn 1)))
    (Default|InitStart _asbp_robot_spawner)))

(event Input|KeyboardEvents|1
  (params (Key :type Key%20Structure :default "None"))
  (:Pressed
    (bind _asbp_robot_spawner (Utilities|Casting|CastToBP_RobotSpawner (Game|Player|GetPlayerPawn 0)))
    (Default|InitStart _asbp_robot_spawner)))

(fn ConstructionScript)