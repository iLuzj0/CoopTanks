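; BP_GameState is a game state that tracks remaining enemies and advances level progress when all are dead.
; GatherEnemies counts every BP_EnemieBase actor, and EnemieDies decrements that count and copies it to each top-level WBP_MainHUD widget.
; At zero, it increments LevelProceeded in BP_GameInstance, removes any additional players with their pawns, and reloads via the RestartLevel console command.
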(event Custom|GatherEnemies
  (bind _outactors (Actor|GetAllActorsOfClass "/Game/Blueprints/Actors/Enemies/BP_EnemieBase.BP_EnemieBase_C"))
  (Variables|Default|SetEnemiesCount (Utilities|Array|Length _outactors)))

(event Custom|EnemieDies
  (bind _returnvalue (Game|GetGameInstance))
  (bind _asbp_game_instance (Utilities|Casting|CastToBP_GameInstance _returnvalue))
  (Math|Integer|DecrementInt (Variables|Default|GetEnemiesCount)
    (:%20%20
      (bind _foundwidgets (Widget|GetAllWidgetsOfClass "/Game/Widgets/HUD/WBP_MainHUD.WBP_MainHUD_C" true))
      (for _array_element _foundwidgets
        (bind _output_get (Variables|/Game/Widgets/HUD/WBP_MainHUD.WBP_MainHUD_C|SetEnemiesCount _array_element (Variables|Default|GetEnemiesCount)))
        (if (== _output_get 0)
          (Variables|/Game/ModularLowPolyRobots/Blueprints/BP_GameInstance.BP_GameInstance_C|SetLevelProceeded _asbp_game_instance (+ (Variables|/Game/ModularLowPolyRobots/Blueprints/BP_GameInstance.BP_GameInstance_C|GetLevelProceeded _asbp_game_instance) 1))
          (for _index (range 1 4)
            (Utilities|IsValid (Game|GetPlayerController _index)
              (:Is%20Valid
                (Class|GameplayStatics|RemovePlayer (Game|GetPlayerController _index) true))))
          (Development|ExecuteConsoleCommand "RestartLevel" 0))))))

(fn ConstructionScript)